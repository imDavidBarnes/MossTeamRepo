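; BP_Button_2 is the second player's half of a two-button puzzle that rewards a crystal.
; Its box trigger outlines the button through custom depth for player index 1, and Interact starts a timeline press that resets after about two seconds unless solved.
; A looping timer checks whether BP_Button_1 is active simultaneously.
; If so, it locks the button, removes the trigger and prompt, and spawns WeightedItemEndPuzzleCrystal at the sprite's location.
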(event OnComponentBeginOverlap(Box)
  (params (OverlappedComponent :type Primitive%20Component%20Object%20Reference) (OtherActor :type Actor%20Object%20Reference) (OtherComp :type Primitive%20Component%20Object%20Reference) (OtherBodyIndex :type Integer) (bFromSweep :type Boolean) (SweepResult :type Hit%20Result%20Structure%20%28by%20ref%29))
  (if (== (Variables|Default|GetCharacterRef) OtherActor)
    (Rendering|SetRenderCustomDepth (Variables|Default|GetCube) true)))

(event OnComponentEndOverlap(Box)
  (params (OverlappedComponent :type Primitive%20Component%20Object%20Reference) (OtherActor :type Actor%20Object%20Reference) (OtherComp :type Primitive%20Component%20Object%20Reference) (OtherBodyIndex :type Integer))
  (if (== (Variables|Default|GetCharacterRef) OtherActor)
    (Rendering|SetRenderCustomDepth (Variables|Default|GetCube) false)))

(event Custom|Is%20Button%201%20Active
  (if (Variables|Default|GetButton%202%20Active?)
    (bind _outactors (Actor|GetAllActorsOfClass "/Game/Jordan/BP_Button_1.BP_Button_1_C"))
    (if (Variables|/Game/Jordan/BP_Button_1.BP_Button_1_C|GetButton1Active? (Utilities|Array|Get(acopy) _outactors))
      (Utilities|FlowControl|DoOnce false
        (:Completed
          (Variables|Default|SetOpened? true)
          (Widget|RemovefromParent (Variables|Default|GetInterref))
          (Variables|Default|SetCanInteract? false)
          (Components|DestroyComponent (Variables|Default|GetBox))
          (Game|SpawnActorfromClass "/Game/David/WeightedItemEndPuzzleCrystal.WeightedItemEndPuzzleCrystal_C" (Math|Transform|MakeTransform (Transformation|GetWorldLocation (Variables|Default|GetPaperSprite)) "0, 0, 0" "1.000000,1.000000,1.000000") "Undefined" 0 1e+01 0))))))

(event EventInteract
  (if (Variables|Default|GetCanInteract?)
    (Variables|Default|SetButton%202%20Active? true)
    (Utilities|FlowControl|DoOnce false :!label _label
      (:Completed
        (bind _buttonmovement (Timeline|ButtonPress PlayFromStart)
          (:Update
            (Transformation|SetRelativeLocation (Variables|Default|GetCube) (Math|Vector|MakeVector _buttonmovement 0.0 0.0) false false)
            (Utilities|FlowControl|Delay 2.0)
            (if (not (Variables|Default|GetOpened?))
              (Utilities|FlowControl|Delay 0.1)
              (bind _buttonmovement_2 (Timeline|Timeline_0 Reverse)
                (:Finished
                  (Transformation|SetRelativeLocation (Variables|Default|GetCube) (Math|Vector|MakeVector _buttonmovement_2 0.0 0.0) false false)
                  (Variables|Default|SetButton%202%20Active? false)
                  (goto _label Reset))))))))))

(event EventBeginPlay
  (Utilities|FlowControl|Delay 1.0)
  (bind _asbp_player_base (Utilities|Casting|CastToBP_Player_Base (Game|GetPlayerCharacter 1)))
  (Variables|Default|SetCharacterRef _asbp_player_base)
  (bind _returnvalue (UserInterface|CreateWidget "/Game/Jordan/Widgets/UI_InteractPrompt.UI_InteractPrompt_C"))
  (Variables|Default|SetInterref _returnvalue)
  (Utilities|Time|SetTimerbyEvent (delegate Custom|Is%20Button%201%20Active) 0.1 true))

(fn ConstructionScript)