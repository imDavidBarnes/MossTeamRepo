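; BP_Spikes is a spike hazard with a Death event and an unconnected sequence for movement and game over.
; The Death event is empty, and nothing starts the SpikeMovement timeline logic, so it never runs.
; That dormant logic lerps the root toward 70 units below its current location on each timeline update.
; A DoOnce then leads to a short delay, the UI_GameOver widget and a game pause.
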(event Custom|Death)

(fn ConstructionScript)