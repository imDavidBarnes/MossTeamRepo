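; Interactable button, the first of a pair with BP_Button_2, that must be active at the same time as its partner.
; Box overlap shows or hides an interact prompt for the player.
; Interact plays a timeline press on the cube, then resets after a delay unless Opened is set.
; A looping timer polls both buttons, permanently setting Opened and disabling interaction once both are active.
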(event OnComponentBeginOverlap(Box)
  (params (OverlappedComponent :type Primitive%20Component%20Object%20Reference) (OtherActor :type Actor%20Object%20Reference) (OtherComp :type Primitive%20Component%20Object%20Reference) (OtherBodyIndex :type Integer) (bFromSweep :type Boolean) (SweepResult :type Hit%20Result%20Structure%20%28by%20ref%29))
  (if (== (Variables|Default|GetCharacterRef) OtherActor)
    (if (Variables|Default|GetCanInteract?)
      (UserInterface|Viewport|AddtoPlayerScreen (Variables|Default|GetInteractRef)))))

(event OnComponentEndOverlap(Box)
  (params (OverlappedComponent :type Primitive%20Component%20Object%20Reference) (OtherActor :type Actor%20Object%20Reference) (OtherComp :type Primitive%20Component%20Object%20Reference) (OtherBodyIndex :type Integer))
  (if (== (Variables|Default|GetCharacterRef) OtherActor)
    (Widget|RemovefromParent (Variables|Default|GetInteractRef))))

(event Custom|Is%20Button%201%20Active
  (if (Variables|Default|GetButton1Active?)
    (bind _outactors (Actor|GetAllActorsOfClass "/Game/Jordan/BP_Button_2.BP_Button_2_C"))
    (if (Variables|/Game/Jordan/BP_Button_2.BP_Button_2_C|GetButton%202%20Active? (Utilities|Array|Get(acopy) _outactors))
      (Utilities|FlowControl|DoOnce false
        (:Completed
          (Variables|Default|SetOpened? true)
          (Widget|RemovefromParent (Variables|Default|GetInteractRef))
          (Variables|Default|SetCanInteract? false))))))

(event EventBeginPlay
  (bind _asbp_player_base (Utilities|Casting|CastToBP_Player_Base (Game|GetPlayerCharacter 0)))
  (Variables|Default|SetCharacterRef _asbp_player_base)
  (bind _returnvalue (UserInterface|CreateWidget "/Game/Jordan/UI_InteractPrompt.UI_InteractPrompt_C"))
  (Variables|Default|SetInteractRef _returnvalue)
  (Utilities|Time|SetTimerbyEvent (delegate Custom|Is%20Button%201%20Active) 0.1 true))

(event EventInteract
  (if (Variables|Default|GetCanInteract?)
    (Variables|Default|SetButton1Active? true)
    (Utilities|FlowControl|DoOnce false :!label _label
      (:Completed
        (bind _buttonmovement (Timeline|ButtonPress PlayFromStart)
          (:Update
            (Transformation|SetRelativeLocation (Variables|Default|GetCube) (Math|Vector|MakeVector _buttonmovement 0.0 0.0) false false)
            (Utilities|FlowControl|Delay 2.0)
            (if (not (Variables|Default|GetOpened?))
              (Utilities|FlowControl|Delay 0.1)
              (bind _buttonmovement_2 (Timeline|Timeline_0 ReverseFromEnd)
                (:Finished
                  (Transformation|SetRelativeLocation (Variables|Default|GetCube) (Math|Vector|MakeVector _buttonmovement_2 0.0 0.0) false false)
                  (Variables|Default|SetButton1Active? false)
                  (goto _label Reset))))))))))

(fn ConstructionScript)