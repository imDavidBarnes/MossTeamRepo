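; PlayerWins_BP is a trigger actor that shows the victory screen when the player reaches it.
; A sphere overlap with a valid BP_Player_Base fires once through a DoOnce.
; It clears the TimerEvent timer on BP_FirstPersonGameMode, then creates the UI_Victory widget, adds it to the viewport and plays its image fade-in animation.
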(event OnComponentBeginOverlap(Sphere)
  (params (OverlappedComponent :type Primitive%20Component%20Object%20Reference) (OtherActor :type Actor%20Object%20Reference) (OtherComp :type Primitive%20Component%20Object%20Reference) (OtherBodyIndex :type Integer) (bFromSweep :type Boolean) (SweepResult :type Hit%20Result%20Structure%20%28by%20ref%29))
  (bind _asbp_player_base (Utilities|Casting|CastToBP_Player_Base OtherActor))
  (Utilities|IsValid _asbp_player_base
    (:Is%20Valid
      (Utilities|FlowControl|DoOnce false
        (:Completed
          (bind _asbp_first_person_game_mode (Utilities|Casting|CastToBP_FirstPersonGameMode (Game|GetGameMode)))
          (Utilities|Time|ClearandInvalidateTimerbyHandle (Variables|/Game/FirstPerson/Blueprints/BP_FirstPersonGameMode.BP_FirstPersonGameMode_C|GetTimerEvent _asbp_first_person_game_mode))
          (bind _returnvalue (UserInterface|CreateWidget "/Game/Jordan/Widgets/UI_Victory.UI_Victory_C"))
          (UserInterface|Viewport|AddtoViewport _returnvalue 0)
          (UserInterface|Animation|PlayAnimation _returnvalue (Variables|/Game/Jordan/Widgets/UI_Victory.UI_Victory_C|GetImageFadeIn _returnvalue) 0.0 1 "Forward" 1.0 false))))))

(event EventBeginPlay)

(event Collision|EventActorBeginOverlap
  (params (OtherActor :type Actor%20Object%20Reference)))

(event EventTick
  (params (DeltaSeconds :type Float%20%28single-precision%29)))

(fn ConstructionScript)