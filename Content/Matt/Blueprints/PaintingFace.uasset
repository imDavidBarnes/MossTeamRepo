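; PaintingFace is a painting puzzle actor whose face sections move into place and reward an end-puzzle crystal.
; Each MoveSection call slides a random piece from a five-section array along X with a timeline, then snaps it into place and removes it.
; A DoOnce-throttled Tick checks all seven pieces, including HeadTop and HeadBottom, roughly every second and spawns the crystal at the Cube once all align.
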(event Custom|MoveSection
  (if (>= (Variables|Default|GetMaxInt) 0)
    (bind _output_get (Variables|Default|SetRandInt (Math|Random|RandomIntegerinRange (Variables|Default|GetMinInt) (Variables|Default|GetMaxInt))))
    (Utilities|IsValid (Utilities|Array|Get(acopy) (Variables|Default|GetSections) _output_get)
      (:Is%20Valid
        (Variables|Default|SetRelative%20Location (Variables|/Script/Engine.SceneComponent|GetRelativeLocation (Utilities|Array|Get(acopy) (Variables|Default|GetSections) _output_get)))
        (bind _alpha (Timeline|Timeline_0 PlayFromStart)
          (:Update
            (Transformation|SetRelativeLocation (Utilities|Array|Get(acopy) (Variables|Default|GetSections) _output_get) (Math|Vector|Lerp(Vector) (Variables|/Script/Engine.SceneComponent|GetRelativeLocation (Utilities|Array|Get(acopy) (Variables|Default|GetSections) _output_get)) (+ (Variables|/Script/Engine.SceneComponent|GetRelativeLocation (Utilities|Array|Get(acopy) (Variables|Default|GetSections) _output_get)) "2.000000,0,0") _alpha) false false))
          (:Finished
            (Transformation|SetRelativeLocation (Utilities|Array|Get(acopy) (Variables|Default|GetSections) _output_get) "0.100000, 0, 0" false false)
            (Utilities|Array|RemoveIndex (Variables|Default|GetSections) (Variables|Default|GetRandInt))
            (Variables|Default|SetMaxInt (- (Variables|Default|GetMaxInt) 1))))))))

(event EventBeginPlay
  (Variables|Default|SetSections (Utilities|Array|MakeArray (Variables|Default|GetHeadNose) (Variables|Default|GetHeadEye) (Variables|Default|GetHeadMouth2) (Variables|Default|GetHeadMouth1) (Variables|Default|GetHeadEyeNose))))

(event EventTick
  (params (DeltaSeconds :type Float%20%28single-precision%29))
  (Utilities|FlowControl|DoOnce false :!label _label
    (:Completed
      (if (Math|Boolean|ANDBoolean (Math|Float|NearlyEqual(Float) (.x (Variables|/Script/Engine.SceneComponent|GetRelativeLocation (Variables|Default|GetHeadTop))) 0.1 0.01) (Math|Float|NearlyEqual(Float) (.x (Variables|/Script/Engine.SceneComponent|GetRelativeLocation (Variables|Default|GetHeadNose))) 0.1 0.01) (Math|Float|NearlyEqual(Float) (.x (Variables|/Script/Engine.SceneComponent|GetRelativeLocation (Variables|Default|GetHeadEye))) 0.1 0.01) (Math|Float|NearlyEqual(Float) (.x (Variables|/Script/Engine.SceneComponent|GetRelativeLocation (Variables|Default|GetHeadMouth2))) 0.1 0.01) (Math|Float|NearlyEqual(Float) (.x (Variables|/Script/Engine.SceneComponent|GetRelativeLocation (Variables|Default|GetHeadBottom))) 0.1 0.01) (Math|Float|NearlyEqual(Float) (.x (Variables|/Script/Engine.SceneComponent|GetRelativeLocation (Variables|Default|GetHeadMouth1))) 0.1 0.01) (Math|Float|NearlyEqual(Float) (.x (Variables|/Script/Engine.SceneComponent|GetRelativeLocation (Variables|Default|GetHeadEyeNose))) 0.1 0.01))
        (Game|SpawnActorfromClass "/Game/David/WeightedItemEndPuzzleCrystal.WeightedItemEndPuzzleCrystal_C" (Math|Transform|MakeTransform (Transformation|GetWorldLocation (Variables|Default|GetCube)) "0, 0, 0" "1.000000,1.000000,1.000000") "Undefined" 0 25.0 0)
        (else
          (Utilities|FlowControl|Delay 1.0)
          (goto _label Reset))))))

(fn ConstructionScript)